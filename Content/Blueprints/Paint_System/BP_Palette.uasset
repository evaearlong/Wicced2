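; BP_Palette is a paint palette actor with seven paint blob components for picking a color by looking at it.
; Each tick, a camera-forward line trace finds the hovered blob, gives it a glow overlay material and, on any hit, clears the others.
; When the player character's StrokeFinished event fires, it broadcasts the highlighted blob's color through ColorSelected.
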(event `self.ReceiveBeginPlay`
  (set `self.BlobArray` (`|MakeArray` (`self.PaintBlob`) (`self.PaintBlob1`) (`self.PaintBlob2`) (`self.PaintBlob3`) (`self.PaintBlob4`) (`self.PaintBlob5`) (`self.PaintBlob6`) :!type "StaticMeshComponent Object Reference"))
  (bind _asbp_third_person_character (cast `/Game/ThirdPerson/Blueprints/BP_ThirdPersonCharacter` (`GameplayStatics.GetPlayerPawn` 0)))
  (add `/Game/ThirdPerson/Blueprints/BP_ThirdPersonCharacter.Stroke Finished` _asbp_third_person_character (delegate `Select Color`)))

(event `Select Color`
  (params (NewParam :type "/Game/ThirdPerson/Blueprints/BP_ThirdPersonCharacter Object Reference"))
  (bind _highlighted_color (`self.Highlighted Color`)
    (:`then`
      (`self.Color Selected` (`PaintBlobComponent.PaintColor` _highlighted_color)))
    (:`else`)))

(event `self.ReceiveTick`
  (params (DeltaSeconds :type "Float (single-precision)"))
  (`self.Highlight Hovered Color`))

(fn `Highlight Hovered Color`
  (bind _returnvalue (`GameplayStatics.GetPlayerCameraManager` 0))
  (bind _returnvalue_2 (`self.K2_GetActorLocation` _returnvalue))
  (bind (_outhit _returnvalue_3) (`KismetSystemLibrary.LineTraceSingle` :`Start` _returnvalue_2 :`End` (+ _returnvalue_2 (* (`self.GetActorForwardVector` _returnvalue) 1500.0)) :`TraceChannel` "TraceTypeQuery1" :`bTraceComplex` true :`bIgnoreSelf` false :`TraceColor` (struct :`R` 0.873138 :`G` 0.44134 :`B` 1.0 :`A` 1.0)))
  (if _returnvalue_3
    (bind _aspaint_blob_component (cast `PaintBlobComponent` (`.HitComponent` (`GameplayStatics.BreakHitResult` _outhit)))
      (:`then`
        (bind _output_get (set `self.Highlighted Color` _aspaint_blob_component))
        (`MeshComponent.SetOverlayMaterial` _output_get "/Game/Art/Materials/M_MagicGlow.M_MagicGlow"))
      (:`CastFailed`
        (set `self.Highlighted Color` null)))
    (for _array_element (`self.BlobArray`)
      (if (!= _array_element (`self.Highlighted Color`))
        (`MeshComponent.SetOverlayMaterial` _array_element null)))
    (else
      (set `self.Highlighted Color` null))))

(fn `UserConstructionScript`)