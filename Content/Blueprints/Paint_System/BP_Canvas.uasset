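; BP_Canvas is a paintable canvas actor that puts the third-person character into a first-person painting mode on overlap.
; Entering locks and positions the player, equips a spawned BP_Palette and binds its color and the character's stroke and back events; exiting reverses the mode.
; Stroke starts trace from the camera, spawn a Niagara effect and pass the hit's collision UV to Painting, which supplies the canvas's dynamic material.
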(event `self.ReceiveBeginPlay`
  (`PaintingComponent.InitializePainting` (`self.Painting`))
  (`PrimitiveComponent.SetMaterial` (`self.Canvas`) 0 (`PaintingComponent.CanvasMID` (`self.Painting`))))

(event `self.ReceiveActorBeginOverlap`
  (params (OtherActor :type "Actor Object Reference"))
  (bind _asbp_third_person_character (cast `/Game/ThirdPerson/Blueprints/BP_ThirdPersonCharacter` OtherActor))
  (if (not (`self.canPaint`))
    (`self.Set Painting Mode` _asbp_third_person_character)
    (add `/Game/ThirdPerson/Blueprints/BP_ThirdPersonCharacter.Player Pressed Back` _asbp_third_person_character (delegate `Exit Painting`))
    (add `/Game/Blueprints/Paint_System/BP_Palette.Color Selected` (`self.Palette`) (delegate `Set Brush Color`))
    (add `/Game/ThirdPerson/Blueprints/BP_ThirdPersonCharacter.Stroke Finished` _asbp_third_person_character (delegate `End Stroke`))
    (add `/Game/ThirdPerson/Blueprints/BP_ThirdPersonCharacter.Stroke Started` _asbp_third_person_character (delegate `Begin Stroke`))))

(event `End Stroke`
  (params (NewParam :type "/Game/ThirdPerson/Blueprints/BP_ThirdPersonCharacter Object Reference"))
  (if (`self.Ongoing Stroke`)
    (set `self.Ongoing Stroke` false)
    (`PaintingComponent.FinishStroke` (`self.Painting`))))

(event `Begin Stroke`
  (bind (_location _outhit) (`self.Get Draw Location`))
  (set `self.Ongoing Stroke` true)
  (`NiagaraFunctionLibrary.SpawnSystemAtLocation` "/Game/Art/Niagara/Niagara_PaintingEffect.Niagara_PaintingEffect" _location)
  (`self.DrawBrush` (`GameplayStatics.FindCollisionUV` _outhit)))

(event `Exit Painting`
  (params (Character :type "/Game/ThirdPerson/Blueprints/BP_ThirdPersonCharacter Object Reference"))
  (`self.Exit Painting Mode` Character))

(event `Set Brush Color`
  (params (Color :type "LinearColor Structure"))
  (`PaintingComponent.ChangeBrushColor` (`self.Painting`) Color))

(fn `DrawBrush`
  (params (DrawLocation :type "Vector2D Structure"))
  (if (`self.canPaint`)
    (`PaintingComponent.PaintAtUV` (`self.Painting`) (`local.drawLocation`))))

(fn `Equip Palette`
  (params (Character :type "WiccedCharacter Object Reference"))
  (bind _returnvalue (`|SpawnActorFromClass` "/Game/Blueprints/Paint_System/BP_Palette.BP_Palette_C" (`KismetMathLibrary.MakeTransform` (0.0 0.0 0.0)) "Undefined" "MultiplyWithRoot" null null))
  (set `self.Palette` _returnvalue)
  (`WiccedCharacter.EquipItem` Character _returnvalue "Palette_L"))

(fn `Exit Painting Mode`
  (params (Character :type "/Game/ThirdPerson/Blueprints/BP_ThirdPersonCharacter Object Reference"))
  (if (`self.canPaint`)
    (set `self.canPaint` false)
    (`/Game/ThirdPerson/Blueprints/BP_ThirdPersonCharacter.ToggleThirdPerson` Character)
    (`/Game/ThirdPerson/Blueprints/BP_ThirdPersonCharacter.Toggle Painting` Character false)
    (`self.Unequip Palette` Character)
    (`/Game/ThirdPerson/Blueprints/BP_ThirdPersonCharacter.Enable Movement` Character)))

(fn `Get Draw Location`
  (returns (Location :type "Vector Structure") (OutHit :type "HitResult Structure"))
  (bind _returnvalue (`GameplayStatics.GetPlayerCameraManager` 0))
  (bind _returnvalue_2 (`self.K2_GetActorLocation` _returnvalue))
  (bind _outhit (`KismetSystemLibrary.LineTraceSingle` :`Start` _returnvalue_2 :`End` (+ _returnvalue_2 (* (`self.GetActorForwardVector` _returnvalue) 1500.0)) :`TraceChannel` "TraceTypeQuery1" :`bTraceComplex` true :`bIgnoreSelf` false))
  (bind (_bblockinghit _binitialoverlap _time _distance _location _impactpoint _normal _impactnormal _physmat _hitactor _hitcomponent) (`GameplayStatics.BreakHitResult` _outhit))
  (if (== _hitcomponent (`self.Canvas`))
    _
    (else
      _))
  (return _location _outhit))

(fn `Set Painting Mode`
  (params (Character :type "/Game/ThirdPerson/Blueprints/BP_ThirdPersonCharacter Object Reference"))
  (bind _characterrotation (`self.CharacterRotation`))
  (set `self.canPaint` true)
  (`/Game/ThirdPerson/Blueprints/BP_ThirdPersonCharacter.ToggleFirstPerson` Character)
  (`/Game/ThirdPerson/Blueprints/BP_ThirdPersonCharacter.Toggle Painting` Character true)
  (`self.Equip Palette` Character)
  (`self.K2_SetActorLocationAndRotation` Character (`SceneComponent.K2_GetComponentLocation` _characterrotation) (`SceneComponent.K2_GetComponentRotation` _characterrotation) false false)
  (`/Game/ThirdPerson/Blueprints/BP_ThirdPersonCharacter.Disable Movement` Character))

(fn `Unequip Palette`
  (params (Character :type "/Game/ThirdPerson/Blueprints/BP_ThirdPersonCharacter Object Reference"))
  (`WiccedCharacter.UnequipItem` Character "LeftHand"))

(fn `UserConstructionScript`)